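; World item actor that can be picked up, with bag-type items doubling as openable containers.
; A collision sphere toggles input and prints prompts: E sends the item data to the overlapping actor and destroys the item, F opens a bag as that actor's second inventory.
; SpawnItem sets item data and copies bag contents from the dropper.
; Bags keep a cell array editable through ChangeCell, and leaving the sphere toggles an open view.
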(event OnComponentBeginOverlap(Sphere)
  (params (OverlappedComponent :type Primitive%20Component%20Object%20Reference) (OtherActor :type Actor%20Object%20Reference) (OtherComp :type Primitive%20Component%20Object%20Reference) (OtherBodyIndex :type Integer) (bFromSweep :type Boolean) (SweepResult :type Hit%20Result%20Structure%20%28by%20ref%29))
  (bind _itemdata (Variables|Default|GetItemData))
  (bind (_name _count _maxcount _stacable _weight _lenght _type) (Utilities|Struct|BreakItem_Data _itemdata))
  ;[1 1 1] При пересечении сферы колизий
  (Variables|Default|SetActor OtherActor)
  (Input|EnableInput (Game|GetPlayerController 0))
  (Development|PrintString (Utilities|String|Append "To pick up " (.Name (Utilities|Struct|BreakItem_Data (Variables|Default|GetItemData))) " press 'E'"))
  (if (Utilities|Enum|Equal(Enum) _type "NewEnumerator6")
    (Development|PrintString (Utilities|String|Append "To open " _name " press \"F\""))
    ;[1 1 1] Изменение размера если предмет впервые обнаружен
    (if (!= (.MaxCount (Utilities|Struct|BreakItem_Data (Variables|Default|GetItemData))) (Utilities|Array|Length (Variables|Default|GetItemInventory)))
      (if (Utilities|Enum|Equal(Enum) (.Type (Utilities|Struct|BreakItem_Data (Variables|Default|GetItemData))) "NewEnumerator6")
        (Utilities|Array|Resize (Variables|Default|GetItemInventory) (.MaxCount (Utilities|Struct|BreakItem_Data (Variables|Default|GetItemData))))))))

(event OnComponentEndOverlap(Sphere)
  (params (OverlappedComponent :type Primitive%20Component%20Object%20Reference) (OtherActor :type Actor%20Object%20Reference) (OtherComp :type Primitive%20Component%20Object%20Reference) (OtherBodyIndex :type Integer))
  ;[1 1 1] При пересечении сферы колизий
  (Variables|Default|SetActor OtherActor)
  (Input|DisableInput (Game|GetPlayerController 0))
  (CallFunction|EndOverlap))

(event Custom|EndOverlap
  ;[1 1 1] Просмотр инвентаря если это сумка
  (if (Variables|Default|GetWidgetOpen)
    (Variables|Default|SetWidgetOpen false)
    (Class|BodySlotInventoryInterfase|ShowSecondInventory(Message) (Variables|Default|GetActor) self)))

(event EventSpawnItem
  (params (itemData :type Item%20Data%20Structure) (HoDrop :type Actor%20Object%20Reference))
  ;[1 1 1] События при спавне
  (bind _output_get (Variables|Default|SetItemData itemData))
  (if (Utilities|Enum|Equal(Enum) (.Type (Utilities|Struct|BreakItem_Data _output_get)) "NewEnumerator6")
    (Utilities|Array|Resize (Variables|Default|GetItemInventory) (.MaxCount (Utilities|Struct|BreakItem_Data _output_get)))
    (bind _inventorybag (Class|BodySlotInventoryInterfase|InventoryBagContent(Message) HoDrop))
    (Variables|Default|SetItemInventory _inventorybag)))

(event EventChangeCell
  (params (CellID :type Integer) (ItemData :type Item%20Data%20Structure))
  (CallFunction|ChangeCellContent CellID ItemData))

(event Input|KeyboardEvents|E
  (params (Key :type Key%20Structure :default "AnyKey"))
  ;[1 1 1] Подбирание рпедмета
  (:Pressed
    (Class|BodySlotInventoryInterfase|ActionWhisHand(Message) (Variables|Default|GetActor) (Utilities|Struct|MakeBodySlotsAction_Struct "NewEnumerator0" (Variables|Default|GetItemData)) self)
    (Actor|DestroyActor)))

(event Input|KeyboardEvents|F
  (params (Key :type Key%20Structure :default "AnyKey"))
  ;[1 1 1] Просмотр инвентаря если это сумка
  (:Pressed
    (if (Utilities|Enum|Equal(Enum) (.Type (Utilities|Struct|BreakItem_Data (Variables|Default|GetItemData))) "NewEnumerator6")
      (Development|PrintString "You open bag" true true "(R=0.019670,G=1.000000,B=0.299929,A=1.000000)")
      (Class|BodySlotInventoryInterfase|ShowSecondInventory(Message) (Variables|Default|GetActor) self)
      (Variables|Default|SetWidgetOpen true))))

(fn ConstructionScript)

(fn ChangeCellContent
  (params (CellID :type Integer) (ItemData :type Item%20Data%20Structure))
  (Utilities|Array|SetArrayElem (Variables|Default|GetItemInventory) CellID ItemData))

(fn ShowItemContent
  (return (Variables|Default|GetItemData) (Variables|Default|GetItemInventory)))