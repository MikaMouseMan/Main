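; BaseHumanoid_BP is a humanoid base Blueprint that holds an eight-slot BodySlots item inventory, exposed through ShowItems.
; ItemAction routes push requests to PushToInventory, which asks ChekPlase for a non-full stackable slot of the same item class.
; PushToInventory writes that slot, normally at max count, and recurses with the leftover count.
; ChekPlase has no separate empty-slot case, and failed pushes only print a message.
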(event EventBeginPlay
  (Utilities|Array|Resize (Variables|Default|GetBody_Slots) 8))

(event Collision|EventActorBeginOverlap
  (params (OtherActor :type Actor%20Object%20Reference)))

(event EventTick
  (params (DeltaSeconds :type Float%20%28single-precision%29)))

(event EventItemAction
  (params (Action :type Action%20Struct%20Structure))
  (bind (_action _itemdata) (Utilities|Struct|BreakAction_Struct Action))
  (switch Utilities|FlowControl|Switch|SwitchonItem_Actions _action
    (:NewEnumerator0
      (CallFunction|PushtoInventory _itemdata))))

(fn ConstructionScript)

(fn PushtoInventory
  (params (ItemData :type Item%20Data%20Structure))
  (LocalVariables|SetL_ItemData ItemData)
  (bind (_slotid _leftcount _canadd) (CallFunction|ChekPlase (LocalVariables|GetL_ItemData)))
  (if _canadd
    (if (< _leftcount 0)
      (Utilities|Array|SetArrayElem (Variables|Default|GetBody_Slots) _slotid (LocalVariables|GetL_ItemData))
      (Development|PrintString "Item added" true true "(R=0.000000,G=1.000000,B=0.077640,A=1.000000)")
      (else
        (Utilities|Array|SetArrayElem (Variables|Default|GetBody_Slots) _slotid (Utilities|Struct|MakeItem_Data (.Name (Utilities|Struct|BreakItem_Data (LocalVariables|GetL_ItemData))) (.MaxCount (Utilities|Struct|BreakItem_Data (LocalVariables|GetL_ItemData))) (.MaxCount (Utilities|Struct|BreakItem_Data (LocalVariables|GetL_ItemData))) (.Stacable (Utilities|Struct|BreakItem_Data (LocalVariables|GetL_ItemData))) (.Weight (Utilities|Struct|BreakItem_Data (LocalVariables|GetL_ItemData))) (.Lenght (Utilities|Struct|BreakItem_Data (LocalVariables|GetL_ItemData))) (.Type (Utilities|Struct|BreakItem_Data (LocalVariables|GetL_ItemData))) (.Icon (Utilities|Struct|BreakItem_Data (LocalVariables|GetL_ItemData))) (.ItemClass (Utilities|Struct|BreakItem_Data (LocalVariables|GetL_ItemData)))))
        ;[1 1 1] Recursion if left item
        (bind _structout (Utilities|Struct|SetmembersinItem_Data (LocalVariables|GetL_ItemData) _leftcount))
        (CallFunction|PushtoInventory _structout)))
    (else
      (Development|PrintString "Cant add" true true "(R=1.000000,G=0.000000,B=0.139431,A=1.000000)"))))

(fn ChekPlase
  (params (itemData :type Item%20Data%20Structure))
  (LocalVariables|SetL_ItemData itemData)
  (bind (_array_element _array_index) (Utilities|Array|ForEachLoopwithBreak (Variables|Default|GetBody_Slots) :!label _label)
    (:LoopBody
      (LocalVariables|SetL_FreeSlotID _array_index)
      ;[1 1 1] Not stack next element
      (if (.Stacable (Utilities|Struct|BreakItem_Data _array_element))
        ;[1 1 1] Check same or not
        (if (== (.ItemClass (Utilities|Struct|BreakItem_Data (LocalVariables|GetL_ItemData))) (.ItemClass (Utilities|Struct|BreakItem_Data (Utilities|Array|Get(acopy) (Variables|Default|GetBody_Slots) (LocalVariables|GetL_FreeSlotID)))))
          ;[1 1 1] Cell is full?
          (if (== (.Count (Utilities|Struct|BreakItem_Data (Utilities|Array|Get(acopy) (Variables|Default|GetBody_Slots) (LocalVariables|GetL_FreeSlotID)))) (.MaxCount (Utilities|Struct|BreakItem_Data (Utilities|Array|Get(acopy) (Variables|Default|GetBody_Slots) (LocalVariables|GetL_FreeSlotID)))))
            (LocalVariables|SetL_CanAdd false)
            (else
              ;[1 1 1] Add if enoght plase
              (if (<= (+ (.Count (Utilities|Struct|BreakItem_Data (LocalVariables|GetL_ItemData))) (.Count (Utilities|Struct|BreakItem_Data (Utilities|Array|Get(acopy) (Variables|Default|GetBody_Slots) (LocalVariables|GetL_FreeSlotID))))) (.MaxCount (Utilities|Struct|BreakItem_Data (Utilities|Array|Get(acopy) (Variables|Default|GetBody_Slots) (LocalVariables|GetL_FreeSlotID)))))
                (LocalVariables|SetL_CanAdd true)
                (LocalVariables|SetL_LeftCount 0)
                (goto _label Break)
                (else
                  ;[1 1 1] If items to much
                  (LocalVariables|SetL_LeftCount (- (.Count (Utilities|Struct|BreakItem_Data (LocalVariables|GetL_ItemData))) (- (.MaxCount (Utilities|Struct|BreakItem_Data (Utilities|Array|Get(acopy) (Variables|Default|GetBody_Slots) (LocalVariables|GetL_FreeSlotID)))) (.Count (Utilities|Struct|BreakItem_Data (Utilities|Array|Get(acopy) (Variables|Default|GetBody_Slots) (LocalVariables|GetL_FreeSlotID)))))))
                  (LocalVariables|SetL_CanAdd true)
                  (goto _label Break)))))
          (else
            (LocalVariables|SetL_CanAdd false)))
        (else
          (LocalVariables|SetL_CanAdd false))))
    (:Completed
      (return (LocalVariables|GetL_FreeSlotID) (LocalVariables|GetL_LeftCount) (LocalVariables|GetL_CanAdd)))))

(fn ShowItems
  (return (Variables|Default|GetBody_Slots)))