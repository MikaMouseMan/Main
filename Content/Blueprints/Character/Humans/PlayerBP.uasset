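; Player-controlled human character Blueprint with first-level input for movement, look, jumping and inventory screens.
; Axis inputs drive movement along the actor's forward and right vectors and controller pitch and yaw, while Space triggers Jump.
; BeginPlay creates the bag and body-slot widgets once, generating the bag's contents.
; The I and C keys use FlipFlops to add or remove the respective widget from the viewport.
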(event EventBeginPlay
  (bind _returnvalue (Game|GetPlayerController 0))
  (|CallParentFunction)
  (bind _returnvalue_2 (UserInterface|CreateWidget "/Game/Blueprints/Widgets/PlayersWidgets/InventoryW_Bag.InventoryW_Bag_C" _returnvalue))
  (bind _output_get (Variables|Default|SetBagInventoryWidget _returnvalue_2))
  (Default|GenerateInventoryWidget _output_get)
  (bind _returnvalue_3 (UserInterface|CreateWidget "/Game/Blueprints/Widgets/PlayersWidgets/InventoryW_BodySlots.InventoryW_BodySlots_C" _returnvalue))
  (Variables|Default|SetBodySlotWidget _returnvalue_3))

(event Input|AxisEvents|InputAxisMouseUpDown
  (params (AxisValue :type Float%20%28single-precision%29))
  ;[1 1 1] Mouse control
  (Pawn|Input|AddControllerPitchInput AxisValue))

(event Input|AxisEvents|InputAxisMouseLeftRight
  (params (AxisValue :type Float%20%28single-precision%29))
  ;[1 1 1] Mouse control
  (Pawn|Input|AddControllerYawInput AxisValue))

(event Input|AxisEvents|InputAxisFBMove
  (params (AxisValue :type Float%20%28single-precision%29))
  ;[1 1 1] Basic control
  (Pawn|Input|AddMovementInput (Transformation|GetActorForwardVector) AxisValue false))

(event Input|AxisEvents|InputAxisLRMove
  (params (AxisValue :type Float%20%28single-precision%29))
  ;[1 1 1] Basic control
  (Pawn|Input|AddMovementInput (Transformation|GetActorRightVector) AxisValue false))

(event Input|KeyboardEvents|C
  (params (Key :type Key%20Structure :default "AnyKey"))
  (bind _bodyslotwidget (Variables|Default|GetBodySlotWidget))
  (:Pressed
    (Utilities|FlowControl|FlipFlop
      (:A
        (UserInterface|Viewport|AddtoViewport _bodyslotwidget 0))
      (:B
        (Widget|RemovefromParent _bodyslotwidget)))))

(event Input|KeyboardEvents|SpaceBar
  (params (Key :type Key%20Structure :default "AnyKey"))
  (:Pressed
    (Character|Jump)))

(event Input|KeyboardEvents|I
  (params (Key :type Key%20Structure :default "AnyKey"))
  (bind _baginventorywidget (Variables|Default|GetBagInventoryWidget))
  (:Pressed
    (Utilities|FlowControl|FlipFlop
      (:A
        (UserInterface|Viewport|AddtoViewport _baginventorywidget 0))
      (:B
        (Widget|RemovefromParent _baginventorywidget)))))

(fn ConstructionScript
  (|CallParentFunction))