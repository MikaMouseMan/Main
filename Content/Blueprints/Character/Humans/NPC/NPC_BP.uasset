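; NPC_BP is a human NPC character Blueprint that offers dialog to actors who come near it.
; Its DialogShere overlaps send interface-style messages telling the other actor that it can or cannot start a dialog, passing itself on entry.
; The AnswerIs event replies to the calling player with dialog data bundling the player, the NPC and its StartDialog text.
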(event OnComponentBeginOverlap(DialogShere)
  (params (OverlappedComponent :type Primitive%20Component%20Object%20Reference) (OtherActor :type Actor%20Object%20Reference) (OtherComp :type Primitive%20Component%20Object%20Reference) (OtherBodyIndex :type Integer) (bFromSweep :type Boolean) (SweepResult :type Hit%20Result%20Structure%20%28by%20ref%29))
  (Class|DialogInterfase|CanStartDialog(Message) OtherActor self))

(event OnComponentEndOverlap(DialogShere)
  (params (OverlappedComponent :type Primitive%20Component%20Object%20Reference) (OtherActor :type Actor%20Object%20Reference) (OtherComp :type Primitive%20Component%20Object%20Reference) (OtherBodyIndex :type Integer))
  (Class|DialogInterfase|CantStartDialog(Message) OtherActor))

(event Collision|EventActorBeginOverlap
  (params (OtherActor :type Actor%20Object%20Reference)))

(event EventTick
  (params (DeltaSeconds :type Float%20%28single-precision%29))
  (|CallParentFunction DeltaSeconds))

(event EventAnswerIs
  (params (ButtonN :type Integer) (From :type Actor%20Object%20Reference))
  ;[1 1 1] Begin
  (Variables|Default|SetPlayer From)
  (Class|DialogInterfase|AnswertoPlayer(Message) (Variables|Default|GetPlayer) (Utilities|Struct|MakeDialogData (Variables|Default|GetPlayer) self (Variables|Default|GetStartDialog))))

(fn ConstructionScript
  (|CallParentFunction))