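; Blacksmith NPC Blueprint that supplies placeholder-like Russian dialog replies for the blacksmith Georgy.
; AnswertoNPC stores the player, pressed button and first answer, then branches on answer depth to send DialogData back through the player's AnswerToPlayerMessage.
; First-level buttons get short replies, and follow-up choices share one path returning to StartDialog.
; Deeper answer levels are unfinished, and the event graph holds only disabled default nodes.
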(event EventBeginPlay
  (|CallParentFunction))

(event Collision|EventActorBeginOverlap
  (params (OtherActor :type Actor%20Object%20Reference)))

(event EventTick
  (params (DeltaSeconds :type Float%20%28single-precision%29))
  (|CallParentFunction DeltaSeconds))

(event EventAnswertoNPC
  (params (ButtonPresed :type Integer) (From :type Actor%20Object%20Reference) (1stAnswer :type Integer) (2ndAnswer :type Integer) (3rdAnswer :type Integer))
  (Variables|Default|SetButtonPressed ButtonPresed)
  (Variables|Default|SetPlayer From)
  (Variables|Default|Set1stAnswer 1stAnswer)
  (if (== (Variables|Default|Get1stAnswer) 0)
    (switch int (Variables|Default|GetButtonPressed)
      (:1
        (Class|DialogInterfase|AnswertoPlayer(Message) (Variables|Default|GetPlayer) (Utilities|Struct|MakeDialogData (Variables|Default|GetPlayer) self (Utilities|Struct|MakeDialogTextData "Кузнец Георгий" "Задать другой вопрос.")) (Variables|Default|GetButtonPressed)))
      (:2
        (Class|DialogInterfase|AnswertoPlayer(Message) (Variables|Default|GetPlayer) (Utilities|Struct|MakeDialogData (Variables|Default|GetPlayer) self (Utilities|Struct|MakeDialogTextData "" "забудь" "" "" "" "" "" "" "" "" " ")) (Variables|Default|GetButtonPressed)))
      (:3
        (Class|DialogInterfase|AnswertoPlayer(Message) (Variables|Default|GetPlayer) (Utilities|Struct|MakeDialogData (Variables|Default|GetPlayer) self (Utilities|Struct|MakeDialogTextData "нет." "\"в начало\"")) (Variables|Default|GetButtonPressed))))
    (elif (== (Variables|Default|Get2ndAnswer) 0)
      (switch int (Variables|Default|Get1stAnswer)
        (:1
          _)
        (:2
          _)
        (:3
          _))
      (switch int (Variables|Default|GetButtonPressed)
        (:0
          ;[1 1 1] Возврат на стартовую
          (Class|DialogInterfase|AnswertoPlayer(Message) (Variables|Default|GetPlayer) (Utilities|Struct|MakeDialogData (Variables|Default|GetPlayer) self (Variables|Default|GetStartDialog)))))
      (elif (== (Variables|Default|Get3rdAnswer) 0)
        _))))

(fn ConstructionScript
  (|CallParentFunction))