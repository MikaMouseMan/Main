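; Player character Blueprint handling movement, mouse look, jumping, a body-slot inventory screen and NPC dialog.
; BeginPlay creates both widgets, and C toggles the inventory through a FlipFlop.
; Dialog events track the available speaker, so E can disable input and open the dialog widget.
; Interface messages relay button choices to the speaker, whose replies update stored answers and the widget, until an exit button restores input.
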(event EventBeginPlay
  (bind _returnvalue (Game|GetPlayerController 0))
  ;[1 1 1] Downloading Widgets
  (|CallParentFunction)
  (bind _returnvalue_2 (UserInterface|CreateWidget "/Game/Blueprints/Widgets/PlayersWidgets/InventoryW_BodySlots.InventoryW_BodySlots_C" _returnvalue))
  (Variables|Default|SetBodySlotWidget _returnvalue_2)
  (bind _returnvalue_3 (UserInterface|CreateWidget "/Game/Blueprints/Widgets/PlayersWidgets/DialogW.DialogW_C" _returnvalue))
  (Variables|Default|SetDialogWidget _returnvalue_3))

(event Input|AxisEvents|InputAxisMouseUpDown
  (params (AxisValue :type Float%20%28single-precision%29))
  ;[1 1 1] Mouse control
  (Pawn|Input|AddControllerPitchInput AxisValue))

(event Input|AxisEvents|InputAxisMouseLeftRight
  (params (AxisValue :type Float%20%28single-precision%29))
  ;[1 1 1] Mouse control
  (Pawn|Input|AddControllerYawInput AxisValue))

(event Input|AxisEvents|InputAxisFBMove
  (params (AxisValue :type Float%20%28single-precision%29))
  ;[1 1 1] Basic control
  (Pawn|Input|AddMovementInput (Transformation|GetActorForwardVector) AxisValue false))

(event Input|AxisEvents|InputAxisLRMove
  (params (AxisValue :type Float%20%28single-precision%29))
  ;[1 1 1] Basic control
  (Pawn|Input|AddMovementInput (Transformation|GetActorRightVector) AxisValue false))

(event Input|KeyboardEvents|SpaceBar
  (params (Key :type Key%20Structure :default "AnyKey"))
  ;[1 1 1] Basic control
  (:Pressed
    (Character|Jump)))

(event Input|KeyboardEvents|C
  (params (Key :type Key%20Structure :default "AnyKey"))
  (bind _bodyslotwidget (Variables|Default|GetBodySlotWidget))
  ;[1 1 1] Show Body interfase
  (:Pressed
    (Utilities|FlowControl|FlipFlop
      (:A
        (UserInterface|Viewport|AddtoViewport _bodyslotwidget 0))
      (:B
        (Widget|RemovefromParent _bodyslotwidget)))))

(event EventAnswerIs
  (params (ButtonN :type Integer) (From :type Actor%20Object%20Reference))
  ;[1 1 1] Dialog
  (if (== ButtonN 11)
    (Widget|RemovefromParent (Variables|Default|GetDialogWidget))
    (Input|EnableInput (Game|GetPlayerController 0))
    (else
      (Class|DialogInterfase|AnswertoNPC(Message) (Variables|Default|GetSpeaker) ButtonN self (Variables|Default|Get1stAnswer) (Variables|Default|Get2ndAnswer) (Variables|Default|Get3rdAnswer)))))

(event EventAnswertoPlayer
  (params (DialogData :type Dialog%20Data%20Structure) (1stAnswer :type Integer) (2ndAnswer :type Integer) (3rdAnswer :type Integer))
  ;[1 1 1] Dialog
  (Variables|Default|Set1stAnswer 1stAnswer)
  (Variables|Default|Set2ndAnswer 2ndAnswer)
  (Variables|Default|Set3rdAnswer 3rdAnswer)
  (Default|UpdateDialog (Variables|Default|GetDialogWidget) DialogData))

(event EventCanStartDialog
  (params (DialogSpeaker :type Actor%20Object%20Reference))
  ;[1 1 1] Dialog
  (Development|PrintString "Can start dialog" true true "(R=0.000000,G=1.000000,B=0.096853,A=1.000000)")
  (Variables|Default|SetCanSpeak true)
  (Variables|Default|SetSpeaker DialogSpeaker))

(event EventCantStartDialog
  ;[1 1 1] Dialog
  (Development|PrintString "Cant Start" true true "(R=1.000000,G=0.000000,B=0.082433,A=1.000000)")
  (Variables|Default|SetCanSpeak false)
  (Variables|Default|SetSpeaker 0))

(event Input|KeyboardEvents|E
  (params (Key :type Key%20Structure :default "AnyKey"))
  ;[1 1 1] Dialog
  ;;[1 1 1] StartDialog
  (:Pressed
    (if (Variables|Default|GetCanSpeak)
      (Input|DisableInput (Game|GetPlayerController 0))
      (UserInterface|Viewport|AddtoViewport (Variables|Default|GetDialogWidget) 0)
      (Class|DialogInterfase|AnswerIs(Message) (stale EventCanStartDialog DialogSpeaker) 0 self))))

(fn ConstructionScript
  (|CallParentFunction))